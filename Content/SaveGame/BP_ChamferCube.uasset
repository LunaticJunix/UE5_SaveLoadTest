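; BP_ChamferCube is a cube actor that triggers saves of player and cube data through messages to the Game Instance.
; When BP_ThirdPersonCharacter overlaps its Sphere, it saves that player's data synchronously, with a shutter sound and printed confirmation.
; A mesh hit starts a looping timer that polls velocity, then clears itself and requests a cube save once the actor nearly stops.
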(event OnComponentBeginOverlap(Sphere)
  (params (OverlappedComponent :type Primitive%20Component%20Object%20Reference) (OtherActor :type Actor%20Object%20Reference) (OtherComp :type Primitive%20Component%20Object%20Reference) (OtherBodyIndex :type Integer) (bFromSweep :type Boolean) (SweepResult :type Hit%20Result%20Structure%20%28by%20ref%29))
  (bind _asbp_third_person_character (Utilities|Casting|CastToBP_ThirdPersonCharacter OtherActor))
  (bind _playersave (Default|GetPlayerSave _asbp_third_person_character))
  (Class|BPISaveGame|SavePlayer(Message) (Game|GetGameInstance) _playersave false)
  (Audio|PlaySound2D "/Engine/VREditor/Sounds/UI/Camera_Shutter.Camera_Shutter" 1.0 1.0 0.0 0 0)
  (Development|PrintString "Saved Player Data"))

(event OnComponentHit(StaticMeshComponent)
  (params (HitComponent :type Primitive%20Component%20Object%20Reference) (OtherActor :type Actor%20Object%20Reference) (OtherComp :type Primitive%20Component%20Object%20Reference) (NormalImpulse :type Vector :default "0, 0, 0") (Hit :type Hit%20Result%20Structure%20%28by%20ref%29))
  (bind _returnvalue (Utilities|Time|SetTimerbyEvent (delegate Custom|CheckVelocity) 0.1 true))
  (Variables|Default|SetCheckVelocityTimer _returnvalue))

(event Custom|CheckVelocity
  (if (< (Math|Vector|VectorLength (Transformation|GetVelocity)) 3.0)
    (Utilities|Time|ClearandInvalidateTimerbyHandle (Variables|Default|GetCheckVelocityTimer))
    (Class|BPISaveGame|SaveCubes(Message) (Game|GetGameInstance) true)))

(event EventBeginPlay)

(event Collision|EventActorBeginOverlap
  (params (OtherActor :type Actor%20Object%20Reference)))

(event EventTick
  (params (DeltaSeconds :type Float%20%28single-precision%29)))

(fn ConstructionScript)